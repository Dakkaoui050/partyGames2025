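; A die actor that rerolls itself about every 15 seconds through a Delay on Tick and prints the face it lands on.
; Each roll moves it to a fixed location with a random rotation, then a recursive check compares its location every 0.2 seconds until it stops moving.
; The result comes from whichever of six numbered face components has its forward vector pointing roughly world up.
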(event `self.ReceiveBeginPlay`)

(event `self.ReceiveTick`
  (params (DeltaSeconds :type "Float (single-precision)"))
  (`KismetSystemLibrary.Delay` 15.0)
  (`self.Rolling`))

(event `Rolling`
  (bind _returnvalue (`KismetMathLibrary.RandomFloatInRange` 0.0 360.0))
  (`self.K2_SetActorLocation` (860.0 670.0 430.0))
  (`self.K2_SetActorRotation` (`KismetMathLibrary.MakeRotator` _returnvalue _returnvalue _returnvalue))
  (`self.Stopped`))

(event `Stopped`
  (set `self.Actorloc` (`self.K2_GetActorLocation`))
  (`KismetSystemLibrary.Delay` 0.2)
  (if (== (`self.Actorloc`) (`self.K2_GetActorLocation`) :`ErrorTolerance` 0.1)
    (`self.Result`)
    (else
      (`self.Stopped`))))

(event `Result`
  (if (== (`SceneComponent.GetForwardVector` (`self.1`)) (0.0 0.0 1.0) :`ErrorTolerance` 0.5)
    (`KismetSystemLibrary.PrintString` "1" true true (struct :`G` 0.66 :`B` 1.0 :`A` 1.0) 5.0)
    (elif (== (`SceneComponent.GetForwardVector` (`self.2`)) (0.0 0.0 1.0) :`ErrorTolerance` 0.5)
      (`KismetSystemLibrary.PrintString` "2" true true (struct :`G` 0.66 :`B` 1.0 :`A` 1.0) 5.0)
      (elif (== (`SceneComponent.GetForwardVector` (`self.3`)) (0.0 0.0 1.0) :`ErrorTolerance` 0.5)
        (`KismetSystemLibrary.PrintString` "3" true true (struct :`G` 0.66 :`B` 1.0 :`A` 1.0) 5.0)
        (elif (== (`SceneComponent.GetForwardVector` (`self.4`)) (0.0 0.0 1.0) :`ErrorTolerance` 0.5)
          (`KismetSystemLibrary.PrintString` "4" true true (struct :`G` 0.66 :`B` 1.0 :`A` 1.0) 5.0)
          (elif (== (`SceneComponent.GetForwardVector` (`self.5`)) (0.0 0.0 1.0) :`ErrorTolerance` 0.5)
            (`KismetSystemLibrary.PrintString` "5" true true (struct :`G` 0.66 :`B` 1.0 :`A` 1.0) 5.0)
            (elif (== (`SceneComponent.GetForwardVector` (`self.6`)) (0.0 0.0 1.0) :`ErrorTolerance` 0.5)
              (`KismetSystemLibrary.PrintString` "6" true true (struct :`G` 0.66 :`B` 1.0 :`A` 1.0) 5.0))))))))

(fn `UserConstructionScript`)